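; BP_AnubisAI is the AI controller for the Anubis character, letting it detect the player by sight.
; It starts the BT_Anubis behavior tree on BeginPlay.
; Sight perception updates for the player pawn write the TargetActor blackboard key, setting it to the player when sensed and clearing it when sight is lost.
; Other senses and actors are ignored.
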(event `self.ReceiveBeginPlay`
  (`self.RunBehaviorTree` "/Game/Characters/AI/BT_Anubis.BT_Anubis"))

(event `self.AIPerception.OnTargetPerceptionUpdated`
  (params (Actor :type "Actor Object Reference") (Stimulus :type "AIStimulus Structure"))
  (bind _returnvalue (`GameplayStatics.GetPlayerPawn` 0))
  (bind _returnvalue_2 (`AIPerceptionSystem.GetSenseClassForStimulus` Stimulus))
  (if (== _returnvalue_2 "/Script/AIModule.AISense_Sight")
    (if (== Actor _returnvalue)
      (`BlackboardComponent.SetValueAsObject` (`AIBlueprintHelperLibrary.GetBlackboard` null) "TargetActor" (select `bool` (`.bSuccessfullySensed` (break `AIStimulus` Stimulus)) :`true` _returnvalue :!type "Object Object Reference")))))

(fn `UserConstructionScript`)